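; Player character Blueprint that adds first-person strafe tilt, a dash, and player, pause and win UI.
; A camera-mode check sets FirstPerson, letting A/D timelines roll the control rotation slightly while moving on the ground.
; Q or E launches the character along its current horizontal velocity, gated by a cooldown.
; It creates the HUD on BeginPlay, pauses into a menu, and checks Win on move input to show the win screen once.
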(event `EnhancedInput|/Game/System/Input/Actions/IA_Camera`
  (params (ActionValue :type Boolean) (ElapsedSeconds :type "Float (double-precision)") (TriggeredSeconds :type "Float (double-precision)") (InputAction :type "InputAction Object Reference" :default "/Game/System/Input/Actions/IA_Camera.IA_Camera"))
  ;[1 1 1] Check if the game is in first person mode, if so set the bool
  (:`Triggered`
    (if (`ActorComponent.IsActive` (`self.FirstPersonCamera`)) :!label _label
      (set `self.bFirstPerson` true)
      (else
        (set `self.bFirstPerson` false)))))

(event `self.ReceiveBeginPlay`
  ;[1 1 1] When game starts, display the player's widget BP
  (bind _returnvalue (`|CreateWidget` "/Game/System/HUD-UI/WBP_Player.WBP_Player_C" (`GameplayStatics.GetPlayerController` 0)))
  (`UserWidget.AddToViewport` _returnvalue 0)
  (goto _label))

(event `Key|D`
  (params (Key :type "Key Structure"))
  (bind _returnvalue (`GameplayStatics.GetPlayerController` 0))
  (bind (_returnvalue_roll _returnvalue_pitch _returnvalue_yaw) (`KismetMathLibrary.BreakRotator` (`Controller.GetControlRotation` _returnvalue)))
  ;[1 1 1] Rotate the camera smoothly when moving sideways, A uses a copy of the same timeline
  (:`Pressed`
    (bind (_direction _newtrack_0) (`Timeline|Camera Rotation for Sideways Movement` :!via `PlayFromStart` :!label _label_2)
      (:`Update`
        (if (and (`NavMovementComponent.IsMovingOnGround` (`self.CustomMovementComponent`)) (`self.bFirstPerson`))
          (`Controller.SetControlRotation` _returnvalue (`KismetMathLibrary.MakeRotator` (`KismetMathLibrary.Lerp` 0.0 2.5 _newtrack_0) _returnvalue_pitch _returnvalue_yaw))))))
  (:`Released`
    (goto _label_2 :!via `Reverse`)))

(event `EnhancedInput|/Game/System/Input/Actions/IA_Pause`
  (params (ActionValue :type Boolean) (ElapsedSeconds :type "Float (double-precision)") (TriggeredSeconds :type "Float (double-precision)") (InputAction :type "InputAction Object Reference" :default "/Game/System/Input/Actions/IA_Pause.IA_Pause"))
  (bind _returnvalue (`GameplayStatics.GetPlayerController` 0))
  ;[1 1 1] Show Pause Menu when the game is paused (P/Esc)
  (:`Started`
    (bind _returnvalue_2 (`|CreateWidget` "/Game/System/HUD-UI/WBP_Pause.WBP_Pause_C"))
    (`UserWidget.AddToViewport` _returnvalue_2 0)
    (set `PlayerController.bShowMouseCursor` true _returnvalue)
    (`WidgetBlueprintLibrary.SetInputMode_UIOnlyEx` _returnvalue null)
    (`GameplayStatics.SetGamePaused` true)))

(event `Key|A`
  (params (Key :type "Key Structure"))
  (bind _returnvalue (`GameplayStatics.GetPlayerController` 0))
  (bind (_returnvalue_roll _returnvalue_pitch _returnvalue_yaw) (`KismetMathLibrary.BreakRotator` (`Controller.GetControlRotation` _returnvalue)))
  ;[1 1 1] Rotate the camera smoothly when moving sideways, A uses a copy of the same timeline
  (:`Pressed`
    (bind (_direction _newtrack_0) (`Timeline|Timeline` :!via `PlayFromStart` :!label _label_3)
      (:`Update`
        (if (and (`NavMovementComponent.IsMovingOnGround` (`self.CustomMovementComponent`)) (`self.bFirstPerson`))
          (`Controller.SetControlRotation` _returnvalue (`KismetMathLibrary.MakeRotator` (`KismetMathLibrary.Lerp` 0.0 -2.5 _newtrack_0) _returnvalue_pitch _returnvalue_yaw))))))
  (:`Released`
    (goto _label_3 :!via `Reverse`)))

(event `Key|Q`
  (params (Key :type "Key Structure"))
  (bind (_returnvalue_x _returnvalue_y) (`KismetMathLibrary.BreakVector` (* (`self.GetVelocity`) 10.0)))
  ;[1 1 1] Dash Ability, Cooldown of 5 seconds
  (:`Pressed`
    (if (not (`self.bIsDashing`)) :!label _label_4
      (set `self.bIsDashing` true)
      (`self.LaunchCharacter` (`KismetMathLibrary.MakeVector` _returnvalue_x _returnvalue_y))
      (`KismetSystemLibrary.Delay` (`self.DashCooldown`))
      (set `self.bIsDashing` false))))

(event `Key|E`
  (params (Key :type "Key Structure"))
  ;[1 1 1] Dash Ability, Cooldown of 5 seconds
  (:`Pressed`
    (goto _label_4)))

(event `EnhancedInput|/Game/System/Input/Actions/IA_Move`
  (params (ActionValue :type "Vector2D Structure") (ElapsedSeconds :type "Float (double-precision)") (TriggeredSeconds :type "Float (double-precision)") (InputAction :type "InputAction Object Reference" :default "/Game/System/Input/Actions/IA_Move.IA_Move"))
  ;[1 1 1] Check for Win Condition
  (:`Triggered`
    (if (`self.bWin`)
      (`/Engine/EditorBlueprintResources/StandardMacros.DoOnce` false
        (:`Completed`
          (bind _returnvalue (`|CreateWidget` "/Game/System/HUD-UI/WBP_Win.WBP_Win_C" (`GameplayStatics.GetPlayerController` 0)))
          (`UserWidget.AddToViewport` _returnvalue 0)
          (`WidgetBlueprintLibrary.SetInputMode_UIOnlyEx` (`GameplayStatics.GetPlayerController` 0) null))))))

(fn `UserConstructionScript`)